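; BP_Block is a breakable block actor that the player can mine over time and collect.
; StartDestroy plays a timeline, paced by DestroyRate, that drives the DestroyAmount parameter on a dynamic material instance, while StopDestroy cancels it and resets the visual.
; When the timeline finishes, the block removes its location from GI_BlockGame, adds its class to the first-person character's inventory and destroys itself.
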(event `self.ReceiveBeginPlay`
  (bind _block (`self.Block`))
  (bind _returnvalue (`PrimitiveComponent.CreateDynamicMaterialInstance` _block 0 (`PrimitiveComponent.GetMaterial` _block 0) "None"))
  (set `self.BlockMat` _returnvalue)
  (`TimelineComponent.SetPlayRate` (`self.DestroyTimeline`) (`self.DestroyRate`)))

(event `Start Destroy`
  (bind (_direction _destroyamount) (`Timeline|DestroyTimeline` :!via `PlayFromStart` :!label _label) ; Update Destroy Amount
    (:`Update`
      (`MaterialInstanceDynamic.SetScalarParameterValue` (`self.BlockMat`) "DestroyAmount" _destroyamount))
    (:`Finished`
      (`/Game/FirstPerson/Blueprints/GI_BlockGame.RemoveBlock` (cast `/Game/FirstPerson/Blueprints/GI_BlockGame` (`GameplayStatics.GetGameInstance`) :!pure true) (`SceneComponent.K2_GetComponentLocation` (`self.DefaultSceneRoot`)))
      (`self.DestroyAndAddToInventory`))))

(event `Stop Destroy`
  (`MaterialInstanceDynamic.SetScalarParameterValue` (`self.BlockMat`) "DestroyAmount" 0.0) ; Reset Destroy Amount
  (goto _label :!via `Stop`))

(fn `DestroyAndAddToInventory`
  (bind _asbp_first_person_character (cast `/Game/FirstPerson/Blueprints/BP_FirstPersonCharacter` (`GameplayStatics.GetPlayerCharacter` 0))
    (:`then`
      (`/Game/FirstPerson/Blueprints/BP_FirstPersonCharacter.AddBlockToInventory` _asbp_first_person_character (`GameplayStatics.GetObjectClass` self)))
    (:`CastFailed`
      _))
  (`self.K2_DestroyActor`))

(fn `UserConstructionScript`)