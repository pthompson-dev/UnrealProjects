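; BP_Block_Magma is a magma block that damages the first-person player character while they overlap its box.
; Entering the box stores the player, applies DamageAmount immediately and starts a looping one-second timer that repeats the damage.
; Leaving the box clears that timer, and other actors are ignored through the character cast.
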(event `self.Box.OnComponentBeginOverlap`
  (params (OverlappedComponent :type "PrimitiveComponent Object Reference") (OtherActor :type "Actor Object Reference") (OtherComp :type "PrimitiveComponent Object Reference") (OtherBodyIndex :type Integer) (bFromSweep :type Boolean) (SweepResult :type "HitResult Structure (by ref)"))
  (bind _asbp_first_person_character (cast `/Game/FirstPerson/Blueprints/BP_FirstPersonCharacter` OtherActor))
  (bind _output_get (set `self.PlayerRef` _asbp_first_person_character))
  (`/Game/FirstPerson/Blueprints/BP_FirstPersonCharacter.Damage` _output_get (`self.Damage Amount`))
  (bind _returnvalue (`KismetSystemLibrary.K2_SetTimerDelegate` (delegate `DamageLoop`) 1.0 true))
  (set `self.DamageTimerHandle` _returnvalue))

(event `DamageLoop`
  (`/Game/FirstPerson/Blueprints/BP_FirstPersonCharacter.Damage` (`self.PlayerRef`) (`self.Damage Amount`)))

(event `self.Box.OnComponentEndOverlap`
  (params (OverlappedComponent :type "PrimitiveComponent Object Reference") (OtherActor :type "Actor Object Reference") (OtherComp :type "PrimitiveComponent Object Reference") (OtherBodyIndex :type Integer))
  (cast `/Game/FirstPerson/Blueprints/BP_FirstPersonCharacter` OtherActor)
  (`KismetSystemLibrary.K2_ClearAndInvalidateTimerHandle` (`self.DamageTimerHandle`)))

(fn `UserConstructionScript`
  (`parent.UserConstructionScript`))