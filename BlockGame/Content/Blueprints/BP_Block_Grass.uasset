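; Grass block Blueprint that can be destroyed over time and added to the inventory.
; BeginPlay sets the timeline rate from DestroyRate and creates dynamic material instances for the block mesh's three material slots.
; StartDestroy animates their DestroyAmount parameter, then removes the block's location through GI_BlockGame and calls DestroyAndAddToInventory.
; StopDestroy cancels the timeline and resets DestroyAmount, so interrupted progress is lost.
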(event `self.ReceiveBeginPlay`
  (bind _block (`self.Block`))
  (`TimelineComponent.SetPlayRate` (`self.DestroyTimeline`) (`self.DestroyRate`))
  (for _index (range 3)
    (bind _returnvalue (`PrimitiveComponent.CreateDynamicMaterialInstance` _block _index (`PrimitiveComponent.GetMaterial` _block _index) "None"))
    (`KismetArrayLibrary.Array_Add` (`self.Materials`) _returnvalue)))

(event `self.Start Destroy`
  (bind (_direction _destroyamount) (`Timeline|Timeline` :!via `PlayFromStart` :!label _label) ; Update Destroy Amount
    (:`Update`
      (`MaterialInstanceDynamic.SetScalarParameterValue` (`self.Materials`) "DestroyAmount" _destroyamount))
    (:`Finished`
      (`/Game/FirstPerson/Blueprints/GI_BlockGame.RemoveBlock` (cast `/Game/FirstPerson/Blueprints/GI_BlockGame` (`GameplayStatics.GetGameInstance`) :!pure true) (`SceneComponent.K2_GetComponentLocation` (`self.DefaultSceneRoot`)))
      (`self.DestroyAndAddToInventory`))))

(event `self.Stop Destroy`
  (`MaterialInstanceDynamic.SetScalarParameterValue` (`self.Materials`) "DestroyAmount" 0.0) ; Reset Destroy Amount
  (goto _label :!via `Stop`))

(fn `UserConstructionScript`
  (`parent.UserConstructionScript`))