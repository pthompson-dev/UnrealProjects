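; AI controller for the drone enemy that runs the BT_Drone behavior tree and caches its BP_Drone from the instigator.
; Each tick it eases the drone's yaw toward the blackboard's MoveToLocation with a small fixed-alpha, frame-rate-dependent lerp.
; When PawnSensing sees a pawn, it turns the eye material orange-red and sets the SeePlayer? blackboard flag, with no reset here.
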(event `self.ReceiveBeginPlay`
  (`self.RunBehaviorTree` "/Game/Drone/BT_Drone.BT_Drone")
  (bind _asbp_drone (cast `/Game/Drone/BP_Drone` (`self.GetInstigator`)))
  (set `self.DroneCharacter` _asbp_drone))

(event `self.ReceiveTick`
  (params (DeltaSeconds :type "Float (single-precision)"))
  (bind _dronecharacter (`self.DroneCharacter`))
  (bind (_returnvalue_roll _returnvalue_pitch _returnvalue_yaw) (`KismetMathLibrary.BreakRotator` (`KismetMathLibrary.RLerp` (`self.K2_GetActorRotation` _dronecharacter) (`KismetMathLibrary.FindLookAtRotation` (`self.K2_GetActorLocation` _dronecharacter) (`BlackboardComponent.GetValueAsVector` (`AIBlueprintHelperLibrary.GetBlackboard` null) "MoveToLocation")) 0.01 true)))
  (`self.K2_SetActorRotation` (`self.DroneCharacter`) (`KismetMathLibrary.MakeRotator` 0.0 0.0 _returnvalue_yaw) false))

(event `self.PawnSensing.OnSeePawn`
  (params (Pawn :type "Pawn Object Reference"))
  (`MaterialInstanceDynamic.SetVectorParameterValue` (`/Game/Drone/BP_Drone.DroneMat` (`self.DroneCharacter`)) "EyeColor" (struct :`R` 1.0 :`G` 0.275348 :`A` 1.0))
  (`BlackboardComponent.SetValueAsBool` (`AIBlueprintHelperLibrary.GetBlackboard` null) "SeePlayer?" true))

(fn `UserConstructionScript`)